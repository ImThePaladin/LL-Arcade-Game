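; Experience orb pickup that pops upward on spawn, then homes in on the player to grant experience.
; The cube's first hit resets its constraint mode and enables the detection radius.
; Player overlap with that radius disables physics and starts projectile homing, with a timeline driving acceleration.
; Hitbox contact destroys the orb after a short random delay; the Destroyed event sends ExperienceValue to the player.
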(event OnComponentHit(Cube)
  (params (HitComponent :type Primitive%20Component%20Object%20Reference) (OtherActor :type Actor%20Object%20Reference) (OtherComp :type Primitive%20Component%20Object%20Reference) (NormalImpulse :type Vector :default "0, 0, 0") (Hit :type Hit%20Result%20Structure%20%28by%20ref%29))
  (Utilities|FlowControl|DoOnce false
    (:Completed
      (Class|PrimitiveComponent|SetConstraintMode (Variables|Default|GetCube) "Default")
      (Collision|SetCollisionEnabled (Variables|Default|GetCube) "QueryAndPhysics")
      (Collision|SetCollisionEnabled (Variables|Default|GetDetectionRadius) "QueryOnly"))))

(event OnComponentBeginOverlap(DetectionRadius)
  (params (OverlappedComponent :type Primitive%20Component%20Object%20Reference) (OtherActor :type Actor%20Object%20Reference) (OtherComp :type Primitive%20Component%20Object%20Reference) (OtherBodyIndex :type Integer) (bFromSweep :type Boolean) (SweepResult :type Hit%20Result%20Structure%20%28by%20ref%29))
  (if (== OtherActor (Game|GetPlayerCharacter 0))
    (Utilities|FlowControl|DoOnce false
      (:Completed
        (Physics|SetSimulatePhysics (Variables|Default|GetCube) false)
        (Collision|SetCollisionResponsetoChannel (Variables|Default|GetCube) "ECC_WorldStatic" "ECR_Ignore")
        (Collision|SetCollisionEnabled (Variables|Default|GetCube) "QueryOnly")
        (Variables|/Script/Engine.ProjectileMovementComponent|SetbIsHomingProjectile (Variables|Default|GetProjectileMovement) true)
        (Variables|/Script/Engine.ProjectileMovementComponent|SetHomingTargetComponent (Variables|Default|GetProjectileMovement) (Variables|/Script/Engine.Actor|GetRootComponent (Game|GetPlayerCharacter 0)))
        (bind _newtrack_0 (Timeline|Timeline Play)
          (:Update
            (Variables|/Script/Engine.ProjectileMovementComponent|SetHomingAccelerationMagnitude (Variables|Default|GetProjectileMovement) _newtrack_0)))))))

(event OnComponentBeginOverlap(ExperienceCubeHitbox)
  (params (OverlappedComponent :type Primitive%20Component%20Object%20Reference) (OtherActor :type Actor%20Object%20Reference) (OtherComp :type Primitive%20Component%20Object%20Reference) (OtherBodyIndex :type Integer) (bFromSweep :type Boolean) (SweepResult :type Hit%20Result%20Structure%20%28by%20ref%29))
  (if (== OtherActor (Game|GetPlayerCharacter 0))
    (Utilities|FlowControl|DoOnce false
      (:Completed
        (Audio|Components|Audio|Stop (Variables|Default|GetTimeline))
        (Variables|/Script/Engine.ProjectileMovementComponent|SetHomingAccelerationMagnitude (Variables|Default|GetProjectileMovement) 9.48e+03)
        (Utilities|FlowControl|Delay (Math|Random|RandomFloatinRange 0.1 0.3))
        (Actor|DestroyActor)))))

(event EventBeginPlay
  (bind _returnvalue (Math|Random|RandomUnitVector))
  (bind _returnvalue_2 (* _returnvalue "0.200000,0.200000,100.000000"))
  (bind (_x _y) (Math|Vector|BreakVector _returnvalue_2))
  (Class|PrimitiveComponent|SetConstraintMode (Variables|Default|GetCube) "None")
  (Physics|AddImpulse (Variables|Default|GetCube) (Math|Vector|MakeVector _x _y (Math|Float|Absolute(Float) (.z (Math|Vector|ClampVectorSize _returnvalue_2 0.45 0.5)))) "None" false))

(event EventDestroyed
  (Class|BPIPlayerInterface|GainExperience(Message) (Game|GetPlayerCharacter 0) (Variables|Default|GetExperienceValue)))

(fn ConstructionScript)