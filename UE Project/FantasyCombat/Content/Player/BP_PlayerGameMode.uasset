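; Player game mode that spawns waves of random enemies at level TargetPoints and counts elapsed seconds.
; On BeginPlay it caches all TargetPoints and starts two looping timers, one for waves every ten seconds and one for the clock.
; Each wave's loop scales with the point count, removing a randomly drawn point after each spawn.
; The working point list is restored from a saved copy after every wave.
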(event Custom|IncrementTimerBy1Second
  (Math|Integer|IncrementInt (Variables|Default|GetTime)))

(event Custom|StartSpawn
  (for _index (range 0 (Math|Integer|Clamp(Integer) (Utilities|Array|Length (Variables|Default|GetSpawnPoints)) 5 (Utilities|Array|Length (Variables|Default|GetSpawnPoints))))
    (CallFunction|SpawnEnemy (.OutItem (Utilities|Array|Random (Variables|Default|GetEnemies)))))
  (Variables|Default|SetSpawnPoints (Variables|Default|GetSpawnPointsRefresher)))

(event Custom|BeginTimer
  (bind _returnvalue (Utilities|Time|SetTimerbyEvent (delegate Custom|IncrementTimerBy1Second) 1.0 true))
  (Variables|Default|SetTimeTimer _returnvalue))

(event Custom|SpawnEnemy
  (params (NewParam :type Actor%20Class%20Reference))
  (bind _spawnpoints (Variables|Default|GetSpawnPoints))
  (bind (_outitem _outindex) (Utilities|Array|Random _spawnpoints))
  (Utilities|IsValid _outitem
    (:Is%20Valid
      (Game|SpawnActorfromClass NewParam (Math|Transform|MakeTransform (Transformation|GetActorLocation _outitem) "0, 0, 0" "1.000000,1.000000,1.000000") "Undefined" "MultiplyWithRoot" 0 0)
      (Utilities|Array|RemoveIndex _spawnpoints _outindex))))

(event EventBeginPlay
  (bind _outactors (Actor|GetAllActorsOfClass "/Script/Engine.TargetPoint"))
  (bind _output_get (Variables|Default|SetSpawnPoints _outactors))
  (Variables|Default|SetSpawnPointsRefresher _output_get)
  (Utilities|Time|SetTimerbyEvent (delegate Custom|StartSpawn) 1e+01 true)
  (CallFunction|BeginTimer))

(fn ConstructionScript)