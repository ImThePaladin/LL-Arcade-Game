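; BP_Goblin is a goblin enemy Blueprint with a mesh and an axe.
; On BeginPlay it runs the parent logic, waits a few seconds, then starts a looping animation on the mesh.
; It then moves the axe to the mesh's weapon socket and attaches it there with snap rules.
; It adds no other behavior, as Tick, overlap and construction hold no logic of their own.
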(event EventBeginPlay
  (|CallParentFunction)
  (Utilities|FlowControl|Delay 3.2)
  (Components|Animation|PlayAnimation (Variables|Character|GetMesh) "/Game/Animations/Goblin/AS_Goblin.AS_Goblin" true)
  (Transformation|SetWorldTransform (Variables|Default|GetAxe) (Transformation|GetSocketTransform (Variables|Character|GetMesh) "WeaponSocket" "RTS_World") false false)
  (Transformation|AttachComponentToComponent (Variables|Default|GetAxe) (Variables|Character|GetMesh) "WeaponSocket" "SnapToTarget" "SnapToTarget" "SnapToTarget" true))

(event Collision|EventActorBeginOverlap
  (params (OtherActor :type Actor%20Object%20Reference)))

(event EventTick
  (params (DeltaSeconds :type Float%20%28single-precision%29)))

(fn ConstructionScript
  (|CallParentFunction))