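; BP_Slime is a slime enemy character that damages the player on contact.
; When its AttackHitbox overlaps an actor tagged Player, the Attack event sends a fixed damage amount to player character 0 through TakeDamageMessage.
; UpdateWalkSpeed sets the movement component's max walk speed, with no caller in this Blueprint.
; Tick and the construction script are empty, and a debug print of the AI controller's name is disconnected.
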(event OnComponentBeginOverlap(AttackHitbox)
  (params (OverlappedComponent :type Primitive%20Component%20Object%20Reference) (OtherActor :type Actor%20Object%20Reference) (OtherComp :type Primitive%20Component%20Object%20Reference) (OtherBodyIndex :type Integer) (bFromSweep :type Boolean) (SweepResult :type Hit%20Result%20Structure%20%28by%20ref%29))
  (if (Actor|ActorHasTag OtherActor "Player")
    (CallFunction|Attack 5.0)))

(event Custom|Attack
  (params (Amount :type Float%20%28double-precision%29))
  (Class|BPIPlayerInterface|TakeDamage(Message) (Game|GetPlayerCharacter 0) Amount))

(event EventTick
  (params (DeltaSeconds :type Float%20%28single-precision%29)))

(fn ConstructionScript)

(fn UpdateWalkSpeed
  (params (NewWalkSpeed :type Float%20%28double-precision%29))
  (Variables|/Script/Engine.CharacterMovementComponent|SetMaxWalkSpeed (Variables|Character|GetCharacterMovement) NewWalkSpeed))