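; BP_Slime is a slime enemy that damages the player on contact and drops an experience orb when destroyed.
; Player overlap with its hitbox triggers an immediate attack and a looping timer that repeats at AttackSpeed intervals, clearing once a tick finds no overlap.
; Attacks send a TakeDamage message to the player, while incoming damage reduces Health and destroys the slime at zero.
; A helper function sets its max walk speed.
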(event OnComponentBeginOverlap(AttackHitbox)
  (params (OverlappedComponent :type Primitive%20Component%20Object%20Reference) (OtherActor :type Actor%20Object%20Reference) (OtherComp :type Primitive%20Component%20Object%20Reference) (OtherBodyIndex :type Integer) (bFromSweep :type Boolean) (SweepResult :type Hit%20Result%20Structure%20%28by%20ref%29))
  (if (Actor|ActorHasTag OtherActor "Player")
    (CallFunction|Attack)
    (bind _returnvalue (Utilities|Time|SetTimerbyEvent (delegate Custom|TryToAttack) (Variables|Default|GetAttackSpeed) true))
    (Variables|Default|SetAttackTimer _returnvalue)))

(event Custom|TryToAttack
  (if (Collision|IsOverlappingActor (Variables|Default|GetAttackHitbox) (Game|GetPlayerCharacter 0) :!class /Script/Engine.PrimitiveComponent)
    (CallFunction|Attack)
    (else
      (Utilities|Time|ClearandInvalidateTimerbyHandle (Variables|Default|GetAttackTimer)))))

(event EventDestroyed
  (Game|SpawnActorfromClass "/Game/Collectable/BP_ExperienceOrb.BP_ExperienceOrb_C" (Math|Transform|MakeTransform (Transformation|GetActorLocation) "0, 0, 0" "1.000000,1.000000,1.000000") "Undefined" "MultiplyWithRoot" 0 0))

(event EventTakeDamage
  (params (Amount :type S%20Damage%20Struct%20Structure))
  (if (<= (- (Variables|Default|GetHealth) (.amount Amount)) 0.0)
    (Actor|DestroyActor)
    (else
      (Variables|Default|SetHealth (- (Variables|Default|GetHealth) (.amount Amount))))))

(fn ConstructionScript)

(fn UpdateWalkSpeed
  (params (NewWalkSpeed :type Float%20%28double-precision%29))
  (Variables|/Script/Engine.CharacterMovementComponent|SetMaxWalkSpeed (Variables|Character|GetCharacterMovement) NewWalkSpeed))

(fn Attack
  (Class|BPIDamageInterface|TakeDamage(Message) (Game|GetPlayerCharacter 0) (Variables|Default|GetDamageInfo)))