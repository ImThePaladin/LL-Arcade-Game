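; BP_Knight is a knight enemy Blueprint that adds an animation and a socketed sword to its parent class.
; Two seconds after the parent BeginPlay, it plays a looping animation directly on the mesh, then moves the Sword to the WeaponSocket and attaches it with snap-to-target rules.
; Damage handling and construction only forward to the parent.
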(event EventBeginPlay
  (|CallParentFunction)
  (Utilities|FlowControl|Delay 2.0)
  (Components|Animation|PlayAnimation (Variables|Character|GetMesh) "/Game/Animations/Knight/AS_Knight.AS_Knight" true)
  (Transformation|SetWorldTransform (Variables|Default|GetSword) (Transformation|GetSocketTransform (Variables|Character|GetMesh) "WeaponSocket" "RTS_World") false false)
  (Transformation|AttachComponentToComponent (Variables|Default|GetSword) (Variables|Character|GetMesh) "WeaponSocket" "SnapToTarget" "SnapToTarget" "SnapToTarget" true))

(event EventTakeDamage
  (params (Amount :type S%20Weapon%20Struct%20Structure))
  (|CallParentFunction Amount))

(fn ConstructionScript
  (|CallParentFunction))