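; Basic melee enemy that rises from underground on spawn, attacks the player and drops an experience orb when destroyed.
; A timeline drives the rise with collision off, then sets the detour AI controller class.
; Hitbox overlap starts a looping attack timer that stops when the player leaves.
; Damage plays severity-based sounds and either kills or applies knockback and a red flash, with Inflation damage enlarging and slowing it once.
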(event OnComponentBeginOverlap(AttackHitbox)
  (params (OverlappedComponent :type Primitive%20Component%20Object%20Reference) (OtherActor :type Actor%20Object%20Reference) (OtherComp :type Primitive%20Component%20Object%20Reference) (OtherBodyIndex :type Integer) (bFromSweep :type Boolean) (SweepResult :type Hit%20Result%20Structure%20%28by%20ref%29))
  (if (and (Actor|ActorHasTag OtherActor "Player") (Variables|Default|GetCanAttack))
    (CallFunction|Attack)
    (bind _returnvalue (Utilities|Time|SetTimerbyEvent (delegate Custom|TryToAttack) (Variables|Default|GetAttackSpeed) true))
    (Variables|Default|SetAttackTimer _returnvalue)
    (Variables|Default|SetCanAttack false)))

(event Custom|TryToAttack
  (if (Collision|IsOverlappingActor (Variables|Default|GetAttackHitbox) (Game|GetPlayerCharacter 0) :!class /Script/Engine.PrimitiveComponent)
    (CallFunction|Attack)
    (else
      (Utilities|Time|ClearandInvalidateTimerbyHandle (Variables|Default|GetAttackTimer))
      (Variables|Default|SetCanAttack true))))

(event EventDestroyed
  (Game|SpawnActorfromClass "/Game/GameplayActors/BP_ExperienceOrb.BP_ExperienceOrb_C" (Math|Transform|MakeTransform (Transformation|GetActorLocation) "0, 0, 0" "1.000000,1.000000,1.000000") "Undefined" "MultiplyWithRoot" 0 25.0 0))

(event EventTakeDamage
  (params (Amount :type S%20Weapon%20Struct%20Structure))
  (bind _mesh (Variables|Character|GetMesh))
  (bind _charactermovement (Variables|Character|GetCharacterMovement))
  (bind _newparam (CallFunction|DecideWhichHurtNoisetoPlay (.damageamount Amount)))
  (Audio|PlaySound2D _newparam 1.0 1.0 0.0 0 0)
  (if (<= (- (Variables|Default|GetHealth) (.damageamount Amount)) 0.0)
    (Actor|DestroyActor)
    (elif (Utilities|Enum|Equal(Enum) (.damagetype Amount) "Inflation")
      (Utilities|FlowControl|Sequence
        (:then_0
          (Utilities|FlowControl|DoOnce false
            (:Completed
              (Transformation|SetActorScale3D (+ (Transformation|GetActorScale3D) "1.000000,1.000000,1.000000"))
              (Variables|/Script/Engine.CharacterMovementComponent|SetMaxWalkSpeed _charactermovement (/ (Variables|/Script/Engine.CharacterMovementComponent|GetMaxWalkSpeed _charactermovement) 3.0)))))
        (:then_1
          (Variables|Default|SetHealth (- (Variables|Default|GetHealth) (.damageamount Amount)) :!label _label)
          (Transformation|SetActorLocation (+ (Transformation|GetActorLocation) (* (Math|Vector|GetForwardVector (Variables|Character|GetMesh)) (* (.knockback (Variables|Default|GetDamageInfo)) -1.0))) true false)
          (Utilities|IsValid _mesh
            (:Is%20Valid
              (Rendering|Material|SetMaterial _mesh 0 "/Game/Materials/BasicMaterials/MI_Red.MI_Red")
              (Rendering|Material|SetMaterial (Variables|Default|GetCylinder) 0 "/Game/Materials/BasicMaterials/MI_Red.MI_Red")
              (Utilities|FlowControl|Delay 0.2)
              (Rendering|Material|SetMaterial _mesh 0 (Variables|Default|GetDefaultMateial))
              (Rendering|Material|SetMaterial (Variables|Default|GetCylinder) 0 (Variables|Default|GetDefaultMateial))))))
      (else
        (goto _label)))))

(event EventBeginPlay
  (bind _returnvalue (Transformation|GetActorLocation))
  (bind _returnvalue_2 (Transformation|GetActorLocation))
  (Collision|SetActorEnableCollision false)
  (bind _output_get (Variables|Default|SetSpawnZ (- (.z _returnvalue) 5e+02)))
  (Transformation|SetActorLocation (Math|Vector|MakeVector (.x _returnvalue) (.y _returnvalue) _output_get) false false)
  (bind _newtrack_0 (Timeline|LerpSpawn Play)
    (:Update
      (Transformation|SetActorLocation (Math|Vector|MakeVector (.x _returnvalue_2) (.y _returnvalue_2) (Math|Float|Lerp (Variables|Default|GetSpawnZ) (+ (Variables|Default|GetSpawnZ) 6e+02) _newtrack_0)) false false))
    (:Finished
      (Collision|SetActorEnableCollision true)
      (Variables|Default|SetAIControllerClass "/Game/Enemies/AI/BP_DetourAI.BP_DetourAI_C"))))

(fn ConstructionScript)

(fn UpdateWalkSpeed
  (params (NewWalkSpeed :type Float%20%28double-precision%29))
  (Variables|/Script/Engine.CharacterMovementComponent|SetMaxWalkSpeed (Variables|Character|GetCharacterMovement) NewWalkSpeed))

(fn Attack
  (Class|BPIDamageInterface|TakeDamage(Message) (Game|GetPlayerCharacter 0) (Variables|Default|GetDamageInfo)))

(fn DecideWhichHurtNoisetoPlay
  (params (Damage :type Float%20%28double-precision%29))
  (if (< Damage 5.0)
    (return "/Game/SFX/hitHurt.hitHurt")
    (elif (< Damage 1e+01)
      (return "/Game/SFX/medium_hit.medium_hit")
      (elif (< Damage 15.0)
        (return "/Game/SFX/critical.critical")))))