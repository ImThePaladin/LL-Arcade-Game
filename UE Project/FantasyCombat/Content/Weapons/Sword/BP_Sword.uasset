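; BP_Sword is a melee weapon that damages BP_BasicEnemy actors overlapping its AttackHitbox.
; PrimaryUse deals fixed damage immediately, unhiding the Cube and hiding the hitbox component after a short delay.
; SecondaryUse plays the sword animation at a rate derived from AttackSpeed, then at its midpoint calls OpenAttackHitbox with the DamageInfo damage and knockback.
; Hits are one-shot overlap queries delivered through TakeDamageMessage; the Cube's show and hide around the secondary hit occur without delay.
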(event EventSecondaryUse
  (params (DamageInfo :type S%20Weapon%20Struct%20Structure) (UseLocation :type Vector :default "0, 0, 0") (UseRotation :type Rotator :default "0, 0, 0"))
  (bind _cube (Variables|Default|GetCube))
  (Variables|/Script/Engine.SkeletalMeshComponent|SetGlobalAnimRateScale (Variables|Default|GetSword_anim_3) (+ (- 1.0 (.attackspeed DamageInfo)) 1e+01))
  (Components|Animation|PlayAnimation (Variables|Default|GetSword_anim_3) (Variables|Default|GetSwordAnimation) false)
  (Utilities|FlowControl|Delay (* (/ (Animation|GetPlayLength (Variables|Default|GetSwordAnimation)) (Variables|/Script/Engine.SkeletalMeshComponent|GetGlobalAnimRateScale (Variables|Default|GetSword_anim_3))) 0.5))
  (Development|SetHiddeninGame _cube false false)
  (CallFunction|OpenAttackHitbox (.damageamount DamageInfo) (.knockback DamageInfo))
  (Development|SetHiddeninGame _cube true false))

(event EventPrimaryUse
  (params (DamageInfo :type S%20Weapon%20Struct%20Structure) (UseLocation :type Vector :default "0, 0, 0") (UseRotation :type Rotator :default "0, 0, 0"))
  (Development|SetHiddeninGame (Variables|Default|GetCube) false false)
  (Utilities|FlowControl|Sequence
    (:then_0
      (Utilities|FlowControl|Delay 0.2)
      (Development|SetHiddeninGame (Variables|Default|GetAttackHitbox) true false))
    (:then_1
      (for _array_element (Collision|GetOverlappingActors (Variables|Default|GetAttackHitbox) "/Game/Enemies/BP_BasicEnemy.BP_BasicEnemy_C" :!class /Script/Engine.PrimitiveComponent)
        (Class|BPIDamageInterface|TakeDamage(Message) _array_element (Utilities|Struct|MakeS_WeaponStruct 0 5.0 "" 0.0 0 0.0))))))

(fn ConstructionScript)

(fn OpenAttackHitbox
  (params (Damage :type Float%20%28double-precision%29) (Knockback :type Float%20%28double-precision%29))
  (for _array_element (Collision|GetOverlappingActors (Variables|Default|GetAttackHitbox) "/Game/Enemies/BP_BasicEnemy.BP_BasicEnemy_C" :!class /Script/Engine.PrimitiveComponent)
    (Class|BPIDamageInterface|TakeDamage(Message) _array_element (Utilities|Struct|MakeS_WeaponStruct 0 Damage "" 0.0 0 Knockback))))