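; BP_Arrow is a bow projectile that damages actors tagged Enemy through its Arrow1 overlap.
; Each hit sends DamageInfo by TakeDamageMessage and decrements its Pierce count, disabling collision and destroying the arrow after a short delay once depleted.
; Non-enemy overlaps destroy it only if OverlappedComponent, the arrow's own component rather than the other one, is WorldStatic.
; An unconnected easter egg that enlarges and destroys the arrow never runs.
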(event OnComponentBeginOverlap(Arrow1)
  (params (OverlappedComponent :type Primitive%20Component%20Object%20Reference) (OtherActor :type Actor%20Object%20Reference) (OtherComp :type Primitive%20Component%20Object%20Reference) (OtherBodyIndex :type Integer) (bFromSweep :type Boolean) (SweepResult :type Hit%20Result%20Structure%20%28by%20ref%29))
  (if (Actor|ActorHasTag OtherActor "Enemy")
    (Class|BPIDamageInterface|TakeDamage(Message) OtherActor (Variables|Default|GetDamageInfo))
    (bind _result (Math|Integer|DecrementInt (.pierce (Variables|Default|GetDamageInfo)))
      (:%20%20
        (if (<= _result 0)
          (Collision|SetCollisionEnabled (Variables|Default|GetArrow1) "NoCollision")
          (Utilities|FlowControl|Delay 0.2)
          (Actor|DestroyActor))))
    (elif (Utilities|Enum|Equal(Enum) (Collision|GetCollisionObjectType OverlappedComponent) "ECC_WorldStatic")
      (Actor|DestroyActor))))

(fn ConstructionScript)