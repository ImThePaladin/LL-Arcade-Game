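; Experience orb pickup that pops out with a random physics impulse, then flies to the player to grant experience.
; Homing starts once it has hit a surface and the player has signalled it via Interact.
; Physics then switches off, and a timeline drives the ProjectileMovement homing acceleration toward player 0.
; Overlapping the player destroys it after a short random delay; the Destroyed event awards experience and plays a pitch-varied sound.
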(event OnComponentHit(Cube)
  (params (HitComponent :type Primitive%20Component%20Object%20Reference) (OtherActor :type Actor%20Object%20Reference) (OtherComp :type Primitive%20Component%20Object%20Reference) (NormalImpulse :type Vector :default "0, 0, 0") (Hit :type Hit%20Result%20Structure%20%28by%20ref%29))
  (Utilities|FlowControl|DoOnce false ; Only need to check once, good for performance
    (:Completed
      (Class|PrimitiveComponent|SetConstraintMode (Variables|Default|GetCube) "Default") ; Forces the cube straight up
      (Variables|Default|SetTouchedGround true)
      (if (CallFunction|GotoPlayer?)
        (CallFunction|ActivateHoming)))))

(event OnComponentBeginOverlap(Cube)
  (params (OverlappedComponent :type Primitive%20Component%20Object%20Reference) (OtherActor :type Actor%20Object%20Reference) (OtherComp :type Primitive%20Component%20Object%20Reference) (OtherBodyIndex :type Integer) (bFromSweep :type Boolean) (SweepResult :type Hit%20Result%20Structure%20%28by%20ref%29))
  (if (== OtherActor (Game|GetPlayerCharacter 0))
    (Utilities|FlowControl|DoOnce false
      (:Completed
        (Audio|Components|Audio|Stop (Variables|Default|GetTimeline))
        (Utilities|FlowControl|Delay (Math|Random|RandomFloatinRange 0.1 0.3))
        (Actor|DestroyActor)))))

(event OnComponentBeginOverlap(PlayerDetectionHitBox)
  (params (OverlappedComponent :type Primitive%20Component%20Object%20Reference) (OtherActor :type Actor%20Object%20Reference) (OtherComp :type Primitive%20Component%20Object%20Reference) (OtherBodyIndex :type Integer) (bFromSweep :type Boolean) (SweepResult :type Hit%20Result%20Structure%20%28by%20ref%29)))

(event Custom|ActivateHoming
  (Physics|SetSimulatePhysics (Variables|Default|GetCube) false)
  (Collision|SetCollisionResponsetoChannel (Variables|Default|GetCube) "ECC_WorldStatic" "ECR_Ignore")
  (Collision|SetCollisionEnabled (Variables|Default|GetCube) "QueryOnly")
  (Variables|/Script/Engine.ProjectileMovementComponent|SetbIsHomingProjectile (Variables|Default|GetProjectileMovement) true)
  (Variables|/Script/Engine.ProjectileMovementComponent|SetHomingTargetComponent (Variables|Default|GetProjectileMovement) (Variables|/Script/Engine.Actor|GetRootComponent (Game|GetPlayerCharacter 0)))
  (bind _newtrack_0 (Timeline|Timeline Play)
    (:Update
      (Variables|/Script/Engine.ProjectileMovementComponent|SetHomingAccelerationMagnitude (Variables|Default|GetProjectileMovement) _newtrack_0))))

(event EventBeginPlay
  (bind _returnvalue (Math|Random|RandomUnitVector))
  (bind _returnvalue_2 (* _returnvalue "0.200000,0.200000,50.000000"))
  (bind (_x _y) (Math|Vector|BreakVector _returnvalue_2))
  (Class|PrimitiveComponent|SetConstraintMode (Variables|Default|GetCube) "None") ; Default Constraint is only on the Z-axis, this is a work around since there is no node to set the default constraint this way
  (Physics|AddImpulse (Variables|Default|GetCube) (Math|Vector|MakeVector _x _y (Math|Float|Absolute(Float) (.z (Math|Vector|ClampVectorSize _returnvalue_2 0.45 0.5)))) "None" false))

(event EventInteract
  (params (Interacter :type Actor%20Object%20Reference))
  (Variables|Default|SetTouchedPlayer true)
  (if (CallFunction|GotoPlayer?)
    (CallFunction|ActivateHoming)))

(event EventDestroyed
  (Class|BPIPlayerInterface|GainExperience(Message) (Game|GetPlayerCharacter 0) (Variables|Default|GetExperienceValue))
  (Audio|PlaySound2D "/Game/SFX/pickupCoin.pickupCoin" 1.0 (Math|Random|RandomFloatinRange 0.9 0.95) 0.0 0 0))

(fn ConstructionScript)

(fn GotoPlayer?
  (if (Math|Boolean|ANDBoolean (Variables|Default|GetTouchedPlayer) (Variables|Default|GetTouchedGround) (not (Audio|Components|Audio|IsPlaying (Variables|Default|GetTimeline))))
    (return true)
    (else
      (return false))))